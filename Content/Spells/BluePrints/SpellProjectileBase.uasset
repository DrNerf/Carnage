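; Base spell projectile actor that flies toward a target location and reports what it hits.
; On spawn it attaches its particle effect and scales the collision sphere, then moves each tick with VInterpTo, without sweeping.
; Any sphere overlap calls the OnHit dispatcher, and the authority multicasts the hit.
; The multicast spawns a fixed fire impact effect, and the authority destroys the actor.
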(event `MulticastHit`
  (`self.Hit`))

(event `self.ReceiveBeginPlay`
  (bind _scale (`self.Scale`))
  (`GameplayStatics.SpawnEmitterAttached` (`self.Projectile`) (`self.DefaultSceneRoot`) "None" (0.0 0.0 0.0) (struct) _scale "KeepRelativeOffset" false)
  (`SceneComponent.SetRelativeScale3D` (`self.Sphere`) _scale))

(event `self.Sphere.OnComponentBeginOverlap`
  (params (OverlappedComponent :type "PrimitiveComponent Object Reference") (OtherActor :type "Actor Object Reference") (OtherComp :type "PrimitiveComponent Object Reference") (OtherBodyIndex :type Integer) (bFromSweep :type Boolean) (SweepResult :type "HitResult Structure (by ref)"))
  (`KismetSystemLibrary.PrintString` "Spell collision")
  (`self.OnHit` OtherActor (`self.K2_GetActorLocation`))
  (`/Engine/EditorBlueprintResources/ActorMacros.Switch Has Authority`
    (:`Authority`
      (`self.MulticastHit`))))

(event `self.ReceiveTick`
  (params (DeltaSeconds :type "Float (single-precision)"))
  (`self.K2_SetActorLocation` (`KismetMathLibrary.VInterpTo` (`self.K2_GetActorLocation`) (`self.TargetLocation`) DeltaSeconds (`self.Speed`))))

(fn `Hit`
  (`KismetSystemLibrary.PrintString` "Spell Hit")
  (`GameplayStatics.SpawnEmitterAtLocation` "/Game/FantasyMagic/Particles/PS_FireImpact.PS_FireImpact" (`self.K2_GetActorLocation`) (struct) (5.0 5.0 5.0) false)
  (`/Engine/EditorBlueprintResources/ActorMacros.Switch Has Authority`
    (:`Authority`
      (`self.K2_DestroyActor`))))

(fn `UserConstructionScript`)